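; Base projectile actor that deals point damage to what it touches, then destroys itself.
; Both the sphere's begin-overlap and the actor's hit event run the same damage-and-destroy logic.
; Hit direction comes from normalizing the X and Y of the trace start-to-end vector.
; Damage amount and type come from variables, and Launcher is passed as both instigator and damage causer.
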(event OnComponentBeginOverlap(Sphere)
  (params (OverlappedComponent :type Primitive%20Component%20Object%20Reference) (OtherActor :type Actor%20Object%20Reference) (OtherComp :type Primitive%20Component%20Object%20Reference) (OtherBodyIndex :type Integer) (bFromSweep :type Boolean) (SweepResult :type Hit%20Result%20Structure%20%28by%20ref%29))
  (bind (_bblockinghit _binitialoverlap _time _distance _location _impactpoint _normal _impactnormal _physmat _hitactor _hitcomponent _hitbonename _bonename _hititem _elementindex _faceindex _tracestart _traceend) (Collision|BreakHitResult SweepResult))
  (bind _launcher (Variables|Default|GetLauncher))
  (bind _returnvalue (- _traceend _tracestart))
  (Game|Damage|ApplyPointDamage OtherActor (Variables|Default|GetDamage) (Math|Vector|Normalize (Math|Vector|MakeVector (.x _returnvalue) (.y _returnvalue) 0.0)) SweepResult _launcher _launcher (Variables|Default|GetDamage%20Type))
  (Actor|DestroyActor))

(event Collision|EventHit
  (params (MyComp :type Primitive%20Component%20Object%20Reference) (Other :type Actor%20Object%20Reference) (OtherComp :type Primitive%20Component%20Object%20Reference) (bSelfMoved :type Boolean) (HitLocation :type Vector :default "0, 0, 0") (HitNormal :type Vector :default "0, 0, 0") (NormalImpulse :type Vector :default "0, 0, 0") (Hit :type Hit%20Result%20Structure%20%28by%20ref%29))
  (bind (_bblockinghit _binitialoverlap _time _distance _location _impactpoint _normal _impactnormal _physmat _hitactor _hitcomponent _hitbonename _bonename _hititem _elementindex _faceindex _tracestart _traceend) (Collision|BreakHitResult Hit))
  (bind _launcher (Variables|Default|GetLauncher))
  (bind _returnvalue (- _traceend _tracestart))
  (Game|Damage|ApplyPointDamage Other (Variables|Default|GetDamage) (Math|Vector|Normalize (Math|Vector|MakeVector (.x _returnvalue) (.y _returnvalue) 0.0)) Hit _launcher _launcher (Variables|Default|GetDamage%20Type))
  (Actor|DestroyActor))

(fn ConstructionScript)