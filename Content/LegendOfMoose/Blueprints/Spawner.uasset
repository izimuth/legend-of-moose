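; Spawner actor that creates an instance of a configurable actor class at its own location and rotation when play begins.
; If the spawned actor is a Character, it also spawns that character's default controller.
; It binds to the spawned actor's OnDestroyed event and, depending on SpawnOnDestroy, either spawns a replacement or clears its stored reference.
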(event Custom|OnDestroyed_Event
  (params (DestroyedActor :type Actor%20Object%20Reference))
  ;[1 1 1] Primary logic
  ;;[1 1 1] Re-spawn actor?
  (if (Variables|Default|GetSpawnOnDestroy)
    (CallFunction|SpawnActor)
    (else
      (Variables|Default|SetSpawned 0))))

(event Custom|SpawnActor
  ;[1 1 1] Primary logic
  ;;[1 1 1] Spawn specified actor
  (bind _returnvalue (Game|SpawnActorfromClass (Variables|Default|GetActorType) (Math|Transform|MakeTransform (Transformation|GetActorLocation) (Transformation|GetActorRotation)) "Undefined" "MultiplyWithRoot" 0 0))
  (bind _output_get (Variables|Default|SetSpawned _returnvalue))
  (Utilities|FlowControl|Sequence
    (:then_0
      ;;[1 1 1] If spawned was pawn, add its controller
      (bind _ascharacter (Utilities|Casting|CastToCharacter _output_get))
      (Pawn|SpawnDefaultController _ascharacter))
    (:then_1
      ;;[1 1 1] Re-spawn actor?
      (Game|AssignOnDestroyed (Variables|Default|GetSpawned) (delegate Custom|OnDestroyed_Event)))))

(event EventBeginPlay
  ;[1 1 1] Spawn on startup
  (CallFunction|SpawnActor))

(fn ConstructionScript)