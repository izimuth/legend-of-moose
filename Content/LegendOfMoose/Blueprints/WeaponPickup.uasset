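; Weapon pickup actor that displays a weapon in the world and can give it to a hero.
; On BeginPlay it takes its static mesh from the assigned Weapon, then spins steadily around its yaw axis every Tick, scaled by delta time.
; GiveToHero adds the Weapon to the hero's inventory, auto-selecting it only if that inventory is empty.
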(event EventTick
  (params (DeltaSeconds :type Float%20%28single-precision%29))
  (Transformation|AddActorLocalRotation (Math|Rotator|MakeRotator 0.0 0.0 (* DeltaSeconds 1e+02)) false false))

(event EventBeginPlay
  (Components|StaticMesh|SetStaticMesh (Variables|Default|GetMesh) (Variables|/Game/LegendOfMoose/Blueprints/Inventory/WeaponInfo.WeaponInfo_C|GetMesh (Variables|Default|GetWeapon))))

(fn ConstructionScript
  (|CallParentFunction))

(fn GivetoHero
  (params (Hero :type Hero%20Character%20Object%20Reference))
  (bind _inventory (Variables|/Game/LegendOfMoose/Blueprints/Hero/HeroCharacter.HeroCharacter_C|GetInventory Hero))
  (Default|AddWeapon _inventory (Variables|Default|GetWeapon) (Default|IsEmpty _inventory)))