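; WeaponChest is a one-time interactable chest that gives its configured weapon to whoever uses it.
; Interact checks CanInteract, which passes until the Used flag is set, then adds the weapon to the user's Inventory with auto-select.
; It then swaps the chest mesh to the open version, sets Used and calls OnInteractionSuccess.
; Interact returns false even on that success path.
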(event EventBeginPlay
  (|CallParentFunction) ; This node is disabled and will not be called.\nDrag off pins to build functionality.
)

(event Collision|EventActorBeginOverlap
  (params (OtherActor :type Actor%20Object%20Reference))
  (|CallParentFunction OtherActor) ; This node is disabled and will not be called.\nDrag off pins to build functionality.
)

(event EventTick
  (params (DeltaSeconds :type Float%20%28single-precision%29))
  (|CallParentFunction DeltaSeconds) ; This node is disabled and will not be called.\nDrag off pins to build functionality.
)

(fn ConstructionScript
  (|CallParentFunction))

(fn CanInteract
  (return (not (Variables|Default|GetUsed))))

(fn Interact
  (params (UsedBy :type Hero%20Character%20Object%20Reference))
  (if (CallFunction|CanInteract)
    (Default|AddWeapon (Variables|/Game/LegendOfMoose/Blueprints/Hero/HeroCharacter.HeroCharacter_C|GetInventory UsedBy) (Variables|Default|GetWeapon) true)
    (Components|StaticMesh|SetStaticMesh (Variables|Default|GetChestMesh) "/Game/ZL_retroCaves/Meshes/decos/m_deco_cave_chestSmall_open.m_deco_cave_chestSmall_open")
    (Variables|Default|SetUsed true)
    (CallFunction|OnInteractionSuccess)
    (return false)))