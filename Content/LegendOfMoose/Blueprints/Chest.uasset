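; Interactable chest that the hero can open once, showing an "Open" prompt.
; On interaction success it plays an opening sound at its location, swaps its static mesh to the open small cave chest model and sets an Opened flag.
; CanInteract returns false once that flag is set, and no item or reward logic runs here.
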(event EventBeginPlay)

(event Collision|EventActorBeginOverlap
  (params (OtherActor :type Actor%20Object%20Reference)))

(event EventTick
  (params (DeltaSeconds :type Float%20%28single-precision%29)))

(event EventOnInteractionSuccess
  (Audio|PlaySoundatLocation "/Game/LegendOfMoose/Sounds/ChestOpen.ChestOpen" (Transformation|GetActorLocation) "0, 0, 0" 1.0 1.0 0.0 0 0 0 0)
  (Components|StaticMesh|SetStaticMesh (Variables|Default|GetChestMesh) "/Game/ZL_retroCaves/Meshes/decos/m_deco_cave_chestSmall_open.m_deco_cave_chestSmall_open")
  (Variables|Default|SetOpened true))

(fn ConstructionScript
  (|CallParentFunction))

(fn GetInteractionPrompt
  (params (Hero :type Hero%20Character%20Object%20Reference))
  (return "Open"))

(fn CanInteract
  (params (Hero :type Hero%20Character%20Object%20Reference))
  (return (not (Variables|Default|GetOpened))))