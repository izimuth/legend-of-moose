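; EnemyCharacter is an enemy that takes hits, gets knocked back, dies and reports contact to the hero.
; An EnemyState enum gates damage, allowing it only while Ready or Attacking.
; Each point-damage hit launches it horizontally along the shot direction and removes one health, then plays a hit-stun montage or a death montage that ends in destruction.
; Overlaps while alive call OnEnemyContact on HeroCharacter, and OnDamageTaken is an empty hook.
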(event Custom|On%20Damage%20Taken)

(event Collision|EventActorBeginOverlap
  (params (OtherActor :type Actor%20Object%20Reference))
  ;[1 1 1] Send contact event to hero
  (if (Utilities|Enum|NotEqual(Enum) (Variables|Default|GetEnemyState) "NewEnumerator3")
    (bind _ashero_character (Utilities|Casting|CastToHeroCharacter OtherActor))
    (Default|OnEnemyContact _ashero_character self)))

(event Game|Damage|EventPointDamage
  (params (Damage :type Float%20%28single-precision%29) (DamageType :type Damage%20Type%20Object%20Reference) (HitLocation :type Vector :default "0, 0, 0") (HitNormal :type Vector :default "0, 0, 0") (HitComponent :type Primitive%20Component%20Object%20Reference) (BoneName :type Name :default "None") (ShotFromDirection :type Vector :default "0, 0, 0") (InstigatedBy :type Controller%20Object%20Reference) (DamageCauser :type Actor%20Object%20Reference) (HitInfo :type Hit%20Result%20Structure%20%28by%20ref%29))
  (bind _mesh (Variables|Character|GetMesh))
  ;[1 1 1] ON damage event
  ;;[1 1 1] Only continue if can be damaged
  (if (CallFunction|CanTakeDamage)
    ;;[1 1 1] Add knockback effect
    (Character|LaunchCharacter (* (Math|Vector|MakeVector (.x ShotFromDirection) (.y ShotFromDirection) 1.0) "1200.000000,1200.000000,0.000000") false false)
    ;;[1 1 1] Reduce health
    (bind _result (Math|Float|DecrementFloat (Variables|Default|GetHealth))
      (:%20%20
        (bind _output_get (Variables|Default|SetHealth _result))
        (if (> _output_get 0.0)
          ;;[1 1 1] Play hit animation if HP > 0
          (Animation|Montage|PlayMontage _mesh (Variables|Default|GetOnHitMontage)
            (:then
              (Variables|Default|SetEnemyState "NewEnumerator2")
              (CallFunction|OnDamageTaken))
            (:OnCompleted
              (Variables|Default|SetEnemyState "NewEnumerator0")))
          (else
            ;;[1 1 1] Play death animation if HP <= 0
            (Animation|Montage|PlayMontage _mesh (Variables|Default|GetOnDeathMontage)
              (:then
                (Variables|Default|SetEnemyState "NewEnumerator3"))
              (:OnCompleted
                (Actor|DestroyActor)))))))))

(fn ConstructionScript)

(fn CanTakeDamage
  (switch Utilities|FlowControl|Switch|SwitchonEnemyStateEnum (Variables|Default|GetEnemyState)
    (:NewEnumerator0
      _)
    (:NewEnumerator1
      _)
    (:NewEnumerator2
      (return false))
    (:NewEnumerator3
      (return false)))
  (return true))