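; Inventory component that holds its owner's weapons and named resources, tracks the selected weapon and fires its projectile.
; Selection broadcasts a weapon-changed event, starts with the first weapon on BeginPlay, and cycles through a wrapped index via previous/next Enhanced Input actions.
; FireProjectile spawns the selected weapon's projectile type with the owning pawn as instigator.
; AddResource writes amounts to a map, but reads the prior total from key "None" rather than the given name.
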(event Input|EnhancedActionEvents|EnhancedInputActionIA_PrevWeapon
  (params (ActionValue :type Boolean) (ElapsedSeconds :type Float%20%28double-precision%29) (TriggeredSeconds :type Float%20%28double-precision%29) (InputAction :type Input%20Action%20Object%20Reference :default "/Game/LegendOfMoose/Input/IA_PrevWeapon.IA_PrevWeapon"))
  (CallFunction|ChangeWeapon -1))

(event Input|EnhancedActionEvents|EnhancedInputActionIA_NextWeapon
  (params (ActionValue :type Boolean) (ElapsedSeconds :type Float%20%28double-precision%29) (TriggeredSeconds :type Float%20%28double-precision%29) (InputAction :type Input%20Action%20Object%20Reference :default "/Game/LegendOfMoose/Input/IA_NextWeapon.IA_NextWeapon"))
  (CallFunction|ChangeWeapon 1))

(event EventBeginPlay
  (bind _weapons (Variables|Default|GetWeapons))
  (bind _output (Utilities|Array|Get(acopy) _weapons))
  (Utilities|IsValid _output
    (:Is%20Valid
      (CallFunction|SelectWeapon _output))))

(fn AddWeapon
  (params (Weapon :type Weapon%20Info%20Object%20Reference) (AutoSelect :type Boolean))
  (bind _weapons (Variables|Default|GetWeapons))
  (bind _returnvalue (Utilities|Array|AddUnique _weapons Weapon))
  (if AutoSelect
    (bind _selected (CallFunction|SelectWeapon (Utilities|Array|Get(acopy) _weapons _returnvalue)))
    (return _selected)
    (else
      (return (Utilities|Array|Get(acopy) _weapons _returnvalue)))))

(fn SelectWeapon
  (params (Weapon :type Weapon%20Info%20Object%20Reference))
  (bind _weapons (Variables|Default|GetWeapons))
  (bind _returnvalue (Utilities|Array|ContainsItem _weapons Weapon))
  (if _returnvalue
    (bind _output_get (Variables|Default|SetSelected Weapon))
    (Default|CallWeaponChanged _output_get))
  (return _output_get _returnvalue))

(fn ChangeWeapon
  (params (Dir :type Integer))
  (bind _weapons (Variables|Default|GetWeapons))
  (CallFunction|SelectWeapon (Utilities|Array|Get(acopy) (Variables|Default|GetWeapons) (Class|KismetMathLibrary|Wrap (+ Dir (Utilities|Array|FindItem _weapons (Variables|Default|GetSelected))) 0 (Utilities|Array|Length _weapons)))))

(fn FireProjectile
  (params (Origin :type Vector) (Rotation :type Rotator))
  (bind _selected (Variables|Default|GetSelected))
  (Utilities|IsValid _selected
    (:Is%20Valid
      (bind _aspawn (Utilities|Casting|CastToPawn (Components|GetOwner)))
      (Game|SpawnActorfromClass (Variables|/Game/LegendOfMoose/Blueprints/Inventory/WeaponInfo.WeaponInfo_C|GetProjectileType _selected) (Math|Transform|MakeTransform Origin Rotation "1.000000,1.000000,1.000000") "Undefined" "MultiplyWithRoot" 0 _aspawn))))

(fn HasSelected
  (bind _selected (Variables|Default|GetSelected))
  (return _selected (Utilities|IsValid _selected)))

(fn CheckWeaponType
  (params (Type :type WeaponType%20Enum :default "NewEnumerator0"))
  (bind _selected (Variables|Default|GetSelected))
  (Utilities|IsValid _selected
    (:Is%20Valid
      (return (Utilities|Enum|Equal(Enum) (Variables|/Game/LegendOfMoose/Blueprints/Inventory/WeaponInfo.WeaponInfo_C|GetType _selected) Type)))
    (:Is%20Not%20Valid
      (return false))))

(fn IsEmpty
  (return (Utilities|Array|IsEmpty (Variables|Default|GetWeapons))))

(fn AddResource
  (params (Name :type Name) (Amount :type Integer))
  (Utilities|Map|Add (Variables|Default|GetResources) Name (+ Amount (.Value (Utilities|Map|Find (Variables|Default|GetResources) "")))))