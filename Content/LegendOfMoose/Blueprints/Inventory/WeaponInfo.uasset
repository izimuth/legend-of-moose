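; WeaponInfo is an inventory Blueprint that describes a weapon's type and magic cost.
; Two query functions classify the weapon as melee or ranged by comparing its Type variable against the first two enum values.
; A mana cost getter returns ManaCost when the weapon is flagged as magic and zero otherwise.
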(fn IsMelee
  (return (Utilities|Enum|Equal(Enum) (Variables|Default|GetType) "NewEnumerator0")))

(fn IsRanged
  (return (Utilities|Enum|Equal(Enum) (Variables|Default|GetType) "NewEnumerator1")))

(fn GetManaCost
  (if (Variables|Default|GetIsMagic)
    (return (Variables|Default|GetManaCost))
    (else
      (return 0.0))))