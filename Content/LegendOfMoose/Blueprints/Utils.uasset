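; Utility functions for Legend of Moose that convert vectors to rotations and compute directions between actors.
; Vector2D to Angle takes the atan2 in degrees with Y negated, adds an offset, and scales an axis vector by it to build a rotator.
; Direction Between normalizes the vector from ActorB to ActorA and scales it by a multiplier.
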(fn Vector2DtoAngle
  (params (Vector :type Vector%202D%20Structure) (AngleOffset :type Float%20%28double-precision%29) (Axis :type Vector))
  (bind _returnvalue (* (.y Vector) -1.0))
  (bind _returnvalue_2 (Class|KismetMathLibrary|DegAtan2 _returnvalue (.x Vector)))
  (bind _returnvalue_3 (+ _returnvalue_2 AngleOffset))
  (bind _returnvalue_4 (* _returnvalue_3 Axis))
  (return (Math|Rotator|MakeRotator (.x _returnvalue_4) (.y _returnvalue_4) (.z _returnvalue_4))))

(fn DirectionBetween
  (params (Actor%20A :type Actor%20Object%20Reference) (Actor%20B :type Actor%20Object%20Reference) (Multiply :type Vector :default "1.000000,1.000000,1.000000"))
  (return (* (Math|Vector|Normalize (- (Transformation|GetActorLocation Actor%20A) (Transformation|GetActorLocation Actor%20B))) Multiply)))