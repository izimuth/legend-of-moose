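; Player hero Character handling movement, melee and ranged attacks, health and mana, interaction and HUD updates.
; A HeroStatus state gates moving, attacking and taking contact damage, which adds knockback and hit stun.
; Montage notifies toggle per-tick sphere-trace sweeps or fire projectiles, using stats from the Inventory's selected weapon.
; Weighted moving averages smooth facing and the offset follow camera, and modular body meshes follow the main mesh's pose.
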(event InventoryUpdated(Inventory)
  (params (Message :type Text) (Icon :type Texture%202D%20Object%20Reference))
  ;[1 1 1] Inventory updated
  (Default|AddMessage (Variables|/Game/LegendOfMoose/UI/MainHUD.MainHUD_C|GetMessageLog (Variables|Default|GetHUD)) Message)
  (Default|UpdateHUD (Variables|Default|GetHUD))
  (Utilities|IsValid Icon
    (:Is%20Valid
      (Default|ShowAlert (Variables|Default|GetAlertIcon) Icon Message))))

(event WeaponChanged(Inventory)
  (params (Weapon :type Weapon%20Info%20Object%20Reference))
  ;[1 1 1] Update weapon model
  (Components|StaticMesh|SetStaticMesh (Variables|Components|GetRightWeapon) (Variables|/Game/LegendOfMoose/Blueprints/Inventory/WeaponInfo.WeaponInfo_C|GetMesh Weapon))
  (Default|SetItemIcon (Variables|Default|GetHUD) Weapon))

(event Custom|On%20Enemy%20Contact
  (params (Enemy :type Enemy%20Character%20Object%20Reference))
  ;[1 1 1] Apply contact damage with enemies
  (if (CallFunction|CanTakeDamage)
    (Variables|Default|SetHeroStatus "NewEnumerator2")
    (CallFunction|AddHealth (Variables|/Game/LegendOfMoose/Blueprints/EnemyCharacter.EnemyCharacter_C|GetContactDamage Enemy))
    (Character|LaunchCharacter (CallFunction|DirectionBetween self Enemy "2400.000000,2400.000000,0.000000") false false)
    (Animation|Montage|PlayMontage (Variables|Character|GetMesh) "/Game/LegendOfMoose/Blueprints/Hero/Hero_OnHit.Hero_OnHit"
      (:OnCompleted
        (Variables|Default|SetHeroStatus "NewEnumerator0")))))

(event Custom|Display%20Message
  (params (Message :type Text))
  (Default|AddMessage (Variables|/Game/LegendOfMoose/UI/MainHUD.MainHUD_C|GetMessageLog (Variables|Default|GetHUD)) Message))

(event Input|EnhancedActionEvents|EnhancedInputActionIA_Move
  (params (ActionValue :type Vector%202D%20Structure) (ElapsedSeconds :type Float%20%28double-precision%29) (TriggeredSeconds :type Float%20%28double-precision%29) (InputAction :type Input%20Action%20Object%20Reference :default "/Game/LegendOfMoose/Input/IA_Move.IA_Move"))
  ;[1 1 1] Move character
  (if (CallFunction|CanMove)
    (CallFunction|Move ActionValue)))

(event Input|EnhancedActionEvents|EnhancedInputActionIA_Attack
  (params (ActionValue :type Boolean) (ElapsedSeconds :type Float%20%28double-precision%29) (TriggeredSeconds :type Float%20%28double-precision%29) (InputAction :type Input%20Action%20Object%20Reference :default "/Game/LegendOfMoose/Input/IA_Attack.IA_Attack"))
  (bind _inventory (Variables|Default|GetInventory))
  (bind _selected (Variables|/Game/LegendOfMoose/Blueprints/Inventory/Inventory.Inventory_C|GetSelected _inventory))
  ;[1 1 1] Perform attack animation
  (if (CallFunction|CanAttack)
    (CallFunction|ConsumeMana (Default|GetManaCost _selected))
    (bind _notifyname (Animation|Montage|PlayMontage (Variables|Character|GetMesh) (Variables|/Game/LegendOfMoose/Blueprints/Inventory/WeaponInfo.WeaponInfo_C|GetAnim _selected) 1.3)
      (:then
        (Variables|Default|SetHeroStatus "NewEnumerator1")
        (Audio|PlaySoundatLocation (Variables|/Game/LegendOfMoose/Blueprints/Inventory/WeaponInfo.WeaponInfo_C|GetSound (Variables|/Game/LegendOfMoose/Blueprints/Inventory/Inventory.Inventory_C|GetSelected (Variables|Default|GetInventory))) (Transformation|GetActorLocation) "0, 0, 0" 1.0 1.0 0.0 0 0 0 0))
      (:OnCompleted
        (Variables|Default|SetHeroStatus "NewEnumerator0"))
      (:OnNotifyBegin
        (switch name _notifyname
          (:AttackSweepStart
            (Variables|Default|SetAttackSweep true))
          (:AttackSweepEnd
            (Variables|Default|SetAttackSweep false))
          (:RangedFire
            (CallFunction|RangedAttack)))))))

(event Input|EnhancedActionEvents|EnhancedInputActionIA_Use
  (params (ActionValue :type Boolean) (ElapsedSeconds :type Float%20%28double-precision%29) (TriggeredSeconds :type Float%20%28double-precision%29) (InputAction :type Input%20Action%20Object%20Reference :default "/Game/LegendOfMoose/Input/IA_Use.IA_Use"))
  (bind _interactiontarget (Variables|Default|GetInteractionTarget))
  ;[1 1 1] Interact with object if available
  (Utilities|IsValid _interactiontarget
    (:Is%20Valid
      (bind _can_use_after (Default|Interact _interactiontarget self))
      (if (not _can_use_after)
        (Default|HidePrompt (Variables|Default|GetAlertIcon))))))

(event EventBeginPlay
  ;[1 1 1] Init Input Mapping
  (bind _asplayer_controller (Utilities|Casting|CastToPlayerController (Pawn|GetController)))
  (Input|AddMappingContext (PlayerController|LocalPlayerSubsystems|GetEnhancedInputLocalPlayerSubsystem _asplayer_controller) "/Game/LegendOfMoose/Input/IMC_Default.IMC_Default" 0 "(bIgnoreAllPressedKeysUntilRelease=True,bForceImmediately=False,bNotifyUserSettings=False)")
  (CallFunction|InitModel)
  (Variables|Default|SetHealth (Variables|Default|GetMaxHealth))
  (Variables|Default|SetMana (Variables|Default|GetMaxMana))
  (CallFunction|InitHUD))

(event EventTick
  (params (DeltaSeconds :type Float%20%28single-precision%29))
  ;[1 1 1] Per-frame work
  (Utilities|FlowControl|Sequence
    (:then_0
      ;;[1 1 1] Update camera position
      (CallFunction|UpdateCameraPosition (+ (Transformation|GetActorLocation) (Variables|Default|GetCameraOffset)) 0.2))
    (:then_1
      ;;[1 1 1] Perform attack hit checks
      (if (Variables|Default|GetAttackSweep)
        (CallFunction|AttackTrace)))))

(event Collision|EventActorBeginOverlap
  (params (OtherActor :type Actor%20Object%20Reference))
  ;[1 1 1] Check for interactable objects
  (bind _asinteractable (Utilities|Casting|CastToInteractable OtherActor))
  (if (Default|CanInteract _asinteractable self)
    (bind _output_get (Variables|Default|SetInteractionTarget _asinteractable))
    (Default|ShowInteractionPrompt (Variables|Default|GetAlertIcon) _output_get "/Game/Images/xbox_btn_a.xbox_btn_a")))

(event Collision|EventActorEndOverlap
  (params (OtherActor :type Actor%20Object%20Reference))
  ;[1 1 1] Check for interactable objects
  (Utilities|Casting|CastToInteractable OtherActor)
  (Variables|Default|SetInteractionTarget 0)
  (Default|HidePrompt (Variables|Default|GetAlertIcon)))

(fn ConstructionScript
  (Variables|Default|SetCameraOffset "0.000000,440.000000,835.000000"))

(fn InitModel
  (Components|SkinnedMesh|SetLeaderPoseComponent (Variables|Components|GetHair) (Variables|Character|GetMesh) false false))

(fn AttackTrace
  (bind _returnvalue (Transformation|GetActorLocation))
  (bind _returnvalue_2 (Pawn|GetController))
  (bind _inventory (Variables|Default|GetInventory))
  (bind _selected (Variables|/Game/LegendOfMoose/Blueprints/Inventory/Inventory.Inventory_C|GetSelected _inventory))
  (bind _outhits (Collision|MultiSphereTraceByChannel _returnvalue (+ _returnvalue (* (Transformation|GetActorForwardVector) (Variables|/Game/LegendOfMoose/Blueprints/Inventory/WeaponInfo.WeaponInfo_C|GetRange _selected))) (Variables|/Game/LegendOfMoose/Blueprints/Inventory/WeaponInfo.WeaponInfo_C|GetTraceRadius _selected) "TraceTypeQuery2" true 0 "ForOneFrame"))
  (for _array_element _outhits
    (Game|Damage|ApplyPointDamage (.HitActor (Collision|BreakHitResult _array_element)) (Variables|/Game/LegendOfMoose/Blueprints/Inventory/WeaponInfo.WeaponInfo_C|GetDamage (Variables|/Game/LegendOfMoose/Blueprints/Inventory/Inventory.Inventory_C|GetSelected (Variables|Default|GetInventory))) (Math|Vector|Normalize (Math|Vector|MakeVector (.x (- (.TraceEnd (Collision|BreakHitResult _array_element)) (.TraceStart (Collision|BreakHitResult _array_element)))) (.y (- (.TraceEnd (Collision|BreakHitResult _array_element)) (.TraceStart (Collision|BreakHitResult _array_element)))) 0.0)) _array_element _returnvalue_2 _returnvalue_2 "/Game/LegendOfMoose/Blueprints/Hero/HeroSwordDmg.HeroSwordDmg_C")
    (Niagara|SpawnSystematLocation "/Game/LegendOfMoose/Effects/HitSparks.HitSparks" (.ImpactPoint (Collision|BreakHitResult _array_element)))
    (Audio|PlaySoundatLocation (Variables|/Game/LegendOfMoose/Blueprints/Inventory/WeaponInfo.WeaponInfo_C|GetHitSound (Variables|/Game/LegendOfMoose/Blueprints/Inventory/Inventory.Inventory_C|GetSelected (Variables|Default|GetInventory))) (Transformation|GetActorLocation) "0, 0, 0" 1.0 1.0 0.0 0 0 0 0)))

(fn Move
  (params (Dir :type Vector%202D%20Structure))
  ;[1 1 1] Smooth direction updates out; removes jank
  (bind _output_get (Variables|Default|SetFacingDir (Math|Vector2D|MakeVector2D (Class|KismetMathLibrary|WeightedMovingAverageFloat (.x Dir) (.x (Variables|Default|GetFacingDir)) 0.2) (Class|KismetMathLibrary|WeightedMovingAverageFloat (.y Dir) (.y (Variables|Default|GetFacingDir)) 0.2))))
  ;[1 1 1] Rotate character
  (Pawn|SetControlRotation (Pawn|GetController) (CallFunction|Vector2DtoAngle _output_get 0.0 "0.000000,0.000000,1.000000"))
  ;[1 1 1] Move character
  (Pawn|Input|AddMovementInput (Transformation|GetActorForwardVector) 1.0 false))

(fn CanAttack
  (switch Utilities|FlowControl|Switch|SwitchonHeroStatus (Variables|Default|GetHeroStatus)
    (:NewEnumerator0
      (return (CallFunction|CanUseWeapon)))
    (:NewEnumerator1
      _)
    (:NewEnumerator2
      _)
    (:NewEnumerator3
      _))
  (return false))

(fn CanMove
  (switch Utilities|FlowControl|Switch|SwitchonHeroStatus (Variables|Default|GetHeroStatus)
    (:NewEnumerator0
      (return true))
    (:NewEnumerator1
      (return (Default|CheckWeaponType (Variables|Default|GetInventory) "NewEnumerator1")))
    (:NewEnumerator2
      _)
    (:NewEnumerator3
      _))
  (return false))

(fn CanTakeDamage
  (switch Utilities|FlowControl|Switch|SwitchonHeroStatus (Variables|Default|GetHeroStatus)
    (:NewEnumerator0
      _)
    (:NewEnumerator1
      _)
    (:NewEnumerator2
      (return false))
    (:NewEnumerator3
      (return false)))
  (return true))

(fn UpdateCameraPosition
  (params (Location :type Vector) (Weight :type Float%20%28double-precision%29))
  (bind _camera (Variables|Components|GetCamera))
  (Transformation|SetWorldLocation _camera (Class|KismetMathLibrary|WeightedMovingAverageFVector Location (Transformation|GetWorldLocation _camera) Weight) false false))

(fn InitHUD
  (bind _asplayer_controller (Utilities|Casting|CastToPlayerController (Pawn|GetController)))
  (Utilities|FlowControl|Sequence
    (:then_0
      (bind _returnvalue (UserInterface|CreateWidget "/Game/LegendOfMoose/UI/MainHUD.MainHUD_C" _asplayer_controller))
      (bind _output_get (Variables|Default|SetHUD _returnvalue))
      (UserInterface|Viewport|AddtoViewport _output_get 0)
      (Default|UpdateHUD _output_get))
    (:then_1
      (bind _returnvalue_2 (UserInterface|CreateWidget "/Game/LegendOfMoose/UI/PlayerIcon.PlayerIcon_C" _asplayer_controller))
      (bind _output_get_2 (Variables|Default|SetAlertIcon _returnvalue_2))
      (UserInterface|Viewport|AddtoViewport _output_get_2 0))))

(fn AddHealth
  (params (Amount :type Float%20%28double-precision%29))
  (bind _output_get (Variables|Default|SetHealth (Math|Float|Clamp(Float) (+ Amount (Variables|Default|GetHealth)) 0.0 (Variables|Default|GetMaxHealth))))
  (Default|UpdateHUD (Variables|Default|GetHUD))
  (if (<= _output_get 0.0)
    (CallFunction|SetDead true))
  (return _output_get))

(fn RangedAttack
  (Default|FireProjectile (Variables|Default|GetInventory) (Transformation|GetSocketLocation (Variables|Components|GetRightWeapon) "FirePoint") (Pawn|GetControlRotation :!class /Script/Engine.Pawn)))

(fn CanUseWeapon
  (bind _inventory (Variables|Default|GetInventory))
  (bind _selected (Variables|/Game/LegendOfMoose/Blueprints/Inventory/Inventory.Inventory_C|GetSelected _inventory))
  (Utilities|IsValid _selected
    (:Is%20Valid
      (if (Variables|/Game/LegendOfMoose/Blueprints/Inventory/WeaponInfo.WeaponInfo_C|GetIsMagic _selected)
        (return (>= (- (Variables|Default|GetMana) (Variables|/Game/LegendOfMoose/Blueprints/Inventory/WeaponInfo.WeaponInfo_C|GetManaCost _selected)) 0.0))
        (else
          (return true))))
    (:Is%20Not%20Valid
      (return false))))

(fn ConsumeMana
  (params (Amount :type Float%20%28double-precision%29))
  (bind _output_get (Variables|Default|SetMana (Math|Float|Clamp(Float) (- (Variables|Default|GetMana) Amount) 0.0 (Variables|Default|GetMaxMana))))
  (Default|UpdateHUD (Variables|Default|GetHUD))
  (return _output_get))

(fn SetDead
  (params (Is%20Dead :type Boolean))
  (bind _asplayer_controller (Utilities|Casting|CastToPlayerController (Pawn|GetController)))
  (bind _output_get (Variables|Default|SetIsDead Is%20Dead))
  (if _output_get
    (Input|DisableInput _asplayer_controller)
    (Default|CallHeroDied self)
    (else
      (Input|EnableInput 0))))