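; Legacy crab enemy character that reacts to point damage with horizontal knockback, hit animations and death.
; Damage only lands while its state is Ready or Attacking, costing one health per hit regardless of damage amount.
; A surviving hit plays a montage in HitStun, then returns to Ready.
; At zero health it enters Dead, plays a death montage, then switches the mesh to physics ragdoll.
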(event EventBeginPlay)

(event Collision|EventActorBeginOverlap
  (params (OtherActor :type Actor%20Object%20Reference)))

(event EventTick
  (params (DeltaSeconds :type Float%20%28single-precision%29)))

(event Game|Damage|EventPointDamage
  (params (Damage :type Float%20%28single-precision%29) (DamageType :type Damage%20Type%20Object%20Reference) (HitLocation :type Vector :default "0, 0, 0") (HitNormal :type Vector :default "0, 0, 0") (HitComponent :type Primitive%20Component%20Object%20Reference) (BoneName :type Name :default "None") (ShotFromDirection :type Vector :default "0, 0, 0") (InstigatedBy :type Controller%20Object%20Reference) (DamageCauser :type Actor%20Object%20Reference) (HitInfo :type Hit%20Result%20Structure%20%28by%20ref%29))
  (bind _mesh (Variables|Character|GetMesh))
  (bind _mesh_2 (Variables|Character|GetMesh))
  ;[1 1 1] ON damage event
  ;;[1 1 1] Only continue if can be damaged
  (if (CallFunction|CanTakeDamage)
    ;;[1 1 1] Add knockback effect
    (Character|LaunchCharacter (* (Math|Vector|MakeVector (.x ShotFromDirection) (.y ShotFromDirection) 1.0) "1200.000000,1200.000000,0.000000") false false)
    ;;[1 1 1] Reduce health
    (bind _result (Math|Float|DecrementFloat (Variables|Default|GetHealth))
      (:%20%20
        (bind _output_get (Variables|Default|SetHealth _result))
        (if (> _output_get 0.0)
          ;;[1 1 1] Play hit animation if HP > 0
          (Animation|Montage|PlayMontage _mesh_2 "/Game/LegendOfMoose/Blueprints/CrabEnemy/EnemyCrab_OnHitMontage.EnemyCrab_OnHitMontage"
            (:then
              (Variables|Default|SetEnemyState "NewEnumerator2"))
            (:OnCompleted
              (Variables|Default|SetEnemyState "NewEnumerator0")))
          (else
            ;;[1 1 1] Play death animation if HP <= 0
            (Animation|Montage|PlayMontage _mesh_2 "/Game/LegendOfMoose/Blueprints/CrabEnemy/EnemyCrab_OnDeath.EnemyCrab_OnDeath"
              (:then
                (Variables|Default|SetEnemyState "NewEnumerator3"))
              (:OnCompleted
                ;;[1 1 1] Turn to ragdoll after dead
                (Collision|SetCollisionProfileName _mesh "Ragdoll" true :!class /Script/Engine.PrimitiveComponent)
                (Components|SkinnedMesh|SetPhysicsAsset _mesh "/Game/RPGMonsterWave2PBR/Mesh/CrabMonster/CrabMonster_PhysicsAsset.CrabMonster_PhysicsAsset" false)
                (Physics|SetSimulatePhysics _mesh true)))))))))

(fn ConstructionScript)

(fn CanTakeDamage
  (switch Utilities|FlowControl|Switch|SwitchonEnemyStateEnum (Variables|Default|GetEnemyState)
    (:NewEnumerator0
      _)
    (:NewEnumerator1
      _)
    (:NewEnumerator2
      (return false))
    (:NewEnumerator3
      (return false)))
  (return true))