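; Crab enemy for Legend of Moose that wanders in short, randomly directed bursts.
; A looping timer alternates through a FlipFlop between picking one of four axis-aligned directions and zeroing the direction to pause.
; Tick feeds that direction into movement input, scaled by move speed and delta time, only while the enemy state is Ready.
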(event Custom|OnDirectionTimer
  ;[1 1 1] Change direction or pause
  (Utilities|FlowControl|FlipFlop
    (:A
      (CallFunction|PickDirection))
    (:B
      (Variables|Default|SetDirection "0, 0, 0"))))

(event EventBeginPlay
  (bind _returnvalue (Utilities|Time|SetTimerbyEvent (delegate Custom|OnDirectionTimer) 1.5 true))
  (Variables|Default|SetMoveTimer _returnvalue))

(event EventTick
  (params (DeltaSeconds :type Float%20%28single-precision%29))
  (switch Utilities|FlowControl|Switch|SwitchonEnemyStateEnum (Variables|Default|GetEnemyState)
    (:NewEnumerator0
      (Pawn|Input|AddMovementInput (Variables|Default|GetDirection) (* DeltaSeconds (Variables|Default|GetMoveSpeed)) false))))

(fn ConstructionScript
  (|CallParentFunction))

(fn PickDirection
  (switch int (Math|Random|RandomIntegerinRange 0 3)
    (:0
      (Variables|Default|SetDirection "0.000000,1.000000,0.000000"))
    (:1
      (Variables|Default|SetDirection "0.000000,-1.000000,0.000000"))
    (:2
      (Variables|Default|SetDirection "1.000000,0.000000,0.000000"))
    (:3
      (Variables|Default|SetDirection "-1.000000,0.000000,0.000000"))))